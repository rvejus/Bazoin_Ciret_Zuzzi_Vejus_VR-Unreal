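; Pressure plate actor that drives a linked Wall, as part of a door system, when something overlaps its trigger box.
; Overlap swaps the plate material and plays a timeline that lowers the plate and sends its alpha to the Wall through DoorInteractMessage.
; The timeline reverses once the box empties, unless PermActivate is set.
; ShowPlate toggles plate visibility and collision, and the construction script positions it from PressureLocation.
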(event OnComponentBeginOverlap(Box)
  (params (OverlappedComponent :type Primitive%20Component%20Object%20Reference) (OtherActor :type Actor%20Object%20Reference) (OtherComp :type Primitive%20Component%20Object%20Reference) (OtherBodyIndex :type Integer) (bFromSweep :type Boolean) (SweepResult :type Hit%20Result%20Structure%20%28by%20ref%29))
  ;[1 1 1] Color Whan Activate or Not
  (Rendering|Material|SetMaterial (Variables|Default|GetPressurePlate) 0 "/Game/LevelPrototyping/Materials/M_Solid.M_Solid")
  (bind _interpol (Timeline|Activate%20Plate%20Timeline Play)
    (:Update
      (Transformation|SetWorldLocation (Variables|Default|GetPressurePlate) (Math|Vector|Lerp(Vector) (Variables|Default|GetOriginalPlateLocation) (Variables|Default|GetTargetPlateLocation) _interpol) false false)
      (Class|DoorInterface|DoorInteract(Message) (Variables|Components|GetWall) _interpol))))

(event OnComponentEndOverlap(Box)
  (params (OverlappedComponent :type Primitive%20Component%20Object%20Reference) (OtherActor :type Actor%20Object%20Reference) (OtherComp :type Primitive%20Component%20Object%20Reference) (OtherBodyIndex :type Integer))
  ;[1 1 1] Color Whan Activate or Not
  (Rendering|Material|SetMaterial (Variables|Default|GetPressurePlate) 0 "/Game/LevelPrototyping/Materials/MI_Solid_Blue.MI_Solid_Blue")
  (if (and (!= (Variables|Modular|GetPermActivate?) true) (== (Utilities|Array|Length (Collision|GetOverlappingActors (Variables|Default|GetBox) 0 :!class /Script/Engine.PrimitiveComponent)) 0))
    (bind _interpol (Timeline|Activate%20Plate%20Timeline Reverse)
      (:Update
        (Transformation|SetWorldLocation (Variables|Default|GetPressurePlate) (Math|Vector|Lerp(Vector) (Variables|Default|GetOriginalPlateLocation) (Variables|Default|GetTargetPlateLocation) _interpol) false false)
        (Class|DoorInterface|DoorInteract(Message) (Variables|Components|GetWall) _interpol)))))

(event EventBeginPlay
  (bind _showplate_ (Variables|Modular|GetShowPlate?))
  (bind _pressureplate (Variables|Default|GetPressurePlate))
  (bind _pressureplate_2 (Variables|Default|GetPressurePlate))
  (bind _returnvalue (Transformation|GetWorldLocation _pressureplate))
  (bind _returnvalue_2 (select _showplate_ "ECR_Block" "ECR_Ignore"))
  ;[1 1 1] Set Plate Location When Activate
  (Variables|Default|SetOriginalPlateLocation _returnvalue)
  (Variables|Default|SetTargetPlateLocation (- _returnvalue "0.000000,0.000000,2.000000"))
  ;[1 1 1] Set Visible and Collision
  (Rendering|SetVisibility (Variables|Default|GetPressurePlate) _showplate_ false)
  (Collision|SetCollisionResponsetoChannel _pressureplate_2 "ECC_Pawn" _returnvalue_2)
  (Collision|SetCollisionResponsetoChannel _pressureplate_2 "ECC_WorldStatic" _returnvalue_2)
  (Collision|SetCollisionResponsetoChannel _pressureplate_2 "ECC_WorldDynamic" _returnvalue_2))

(fn ConstructionScript
  (Transformation|SetRelativeLocation (Variables|Default|GetPressurePlate) (Variables|SetLocation|GetPressureLocation) false false))