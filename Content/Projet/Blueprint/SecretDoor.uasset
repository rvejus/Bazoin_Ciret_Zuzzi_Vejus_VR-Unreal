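; SecretDoor is a door actor that opens and closes when its DoorInteract event is called.
; The IsOpen flag selects whether a Timeline plays from the start or reverses from the end.
; The timeline's PosDoor track drives a Z lerp of the Door between PosInit and PosOpen.
; The logic also flips IsOpen and plays a 2D door sound, with a DoOnce gate in the chain.
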(event EventBeginPlay)

(event Collision|EventActorBeginOverlap
  (params (OtherActor :type Actor%20Object%20Reference)))

(event EventDoorInteract
  (params (Timeline%20alpha%28interpol%29 :type Float%20%28double-precision%29))
  (if (Variables|Default|GetIsOpen)
    (bind _posdoor (Timeline|Timeline ReverseFromEnd)
      (:Update
        (Utilities|FlowControl|DoOnce false :!label _label
          (:Completed
            (Transformation|SetRelativeLocation (Variables|Default|GetDoor) (Math|Vector|MakeVector 0.0 0.0 (Math|Float|Lerp (Variables|Default|GetPosInit) (Variables|Default|GetPosOpen) _posdoor)) false false)
            (Variables|Default|SetIsOpen (not (Variables|Default|GetIsOpen)))
            (Audio|PlaySound2D "/Game/Projet/Sound/opening_Door.opening_Door" 1.0 1.0 0.0 0 0)
            (goto _label Reset)))))
    (else
      (Timeline|Timeline PlayFromStart))))

(fn ConstructionScript)