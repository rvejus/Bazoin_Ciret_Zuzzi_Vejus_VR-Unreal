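; VR door Blueprint that a motion controller can grab by the handle and swing open, with a keyhole lock.
; Grab stores the controller if it is within the handle's collision sphere, and Release clears it.
; Each Tick, the door locks only if fully closed with KeyHole not unlocked.
; When unlocked, its yaw follows the hand via look-at rotation, clamped to ±90°, and snaps shut when released nearly closed.
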(event EventTick
  (params (DeltaSeconds :type Float%20%28single-precision%29))
  (bind _hand (Variables|Default|GetHand))
  (bind _door (Variables|Default|GetDoor))
  (Utilities|FlowControl|Sequence
    (:then_0
      ;[1 1 1] Check si la porte est verouillé
      (if (and (not (Variables|/Game/Projet/Blueprint/KeyHole.KeyHole_C|GetUnlocked (Variables|Default|GetKeyHole))) (Math|Float|NearlyEqual(Float) (.yaw (Transformation|GetWorldRotation (Variables|Default|GetDoor))) 0.0 1e-06))
        (Variables|Default|SetLocked true)
        (else
          (Variables|Default|SetLocked false))))
    (:then_1
      ;[1 1 1] On ouvre la porte
      (if (not (Variables|Default|GetLocked))
        (Utilities|IsValid _hand
          (:Is%20Valid
            (Transformation|SetWorldRotation _door (Math|Rotator|MakeRotator 0.0 0.0 (Math|Float|ClampAngle (- (.yaw (Math|Rotator|FindLookatRotation (Transformation|GetWorldLocation _hand) (Transformation|GetWorldLocation _door))) 9e+01) -9e+01 9e+01)) false false))
          (:Is%20Not%20Valid
            (if (Math|Float|NearlyEqual(Float) (.yaw (Transformation|GetWorldRotation _door)) 0.0 1e+01)
              (Transformation|SetWorldRotation _door "0, 0, 0" false false))))))))

(event EventGrab
  (params (Motion%20Controller :type Motion%20Controller%20Component%20Object%20Reference))
  (bind _handle_collision (Variables|Default|GetHandle%20collision))
  (if (Utilities|Operators|EqualEqual (Transformation|GetWorldLocation Motion%20Controller) (Transformation|GetWorldLocation _handle_collision) (Variables|/Script/Engine.SphereComponent|GetSphereRadius _handle_collision))
    (Variables|Default|SetHand Motion%20Controller)))

(event EventRelease
  (params (Motion%20Controller :type Motion%20Controller%20Component%20Object%20Reference))
  (if (== Motion%20Controller (Variables|Default|GetHand))
    (Variables|Default|SetHand 0)))

(fn ConstructionScript)